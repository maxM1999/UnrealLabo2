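; SwatGuy character Blueprint that handles the player's HUD and game-over presentation.
; On BeginPlay it creates health bar and potion widgets, sets the portrait, and overrides audio listener attenuation to the character's mesh.
; Health and item-count events refresh those widgets.
; On death it shows the GameOver widget, removes the health bar and reveals the mouse cursor for clicking.
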(event `self.ReceiveBeginPlay`
  (`|ExecutionSequence`
    (:`then_0`
      ;[1 1 1] Construire et afficher les widgets de vie et de potion
      (bind _asplayer_controller (cast `PlayerController` (`self.GetController`)))
      (bind _returnvalue (`|CreateWidget` "/Game/UI/WBP_HealthBar.WBP_HealthBar_C" _asplayer_controller))
      (bind _output_get (set `self.HealthBarWidget` _returnvalue))
      (`UserWidget.AddToViewport` _output_get 0)
      (bind _returnvalue_2 (`|CreateWidget` "/Game/UI/WBP_Potions.WBP_Potions_C" _asplayer_controller))
      (bind _output_get_2 (set `self.PotionWidget` _returnvalue_2))
      (`UserWidget.AddToViewport` _output_get_2 0))
    (:`then_1`
      ;[1 1 1] Assigner l'image du portrait au widget de la barre de vie
      (`Image.SetBrushFromTexture` (`/Game/UI/WBP_HealthBar.Portrait` (`self.HealthBarWidget`)) (`self.GetPortrait`) false))
    (:`then_2`
      ;[1 1 1] Mettre l'audio listener sur le mesh
      (bind _asplayer_controller_2 (cast `PlayerController` (`self.GetController`)))
      (`PlayerController.SetAudioListenerAttenuationOverride` _asplayer_controller_2 (`self.Mesh`) (0.0 0.0 0.0)))))

(event `self.OnUpdateHealth`
  ;[1 1 1] Ajuster le % de la barre de vie
  (`ProgressBar.SetPercent` (`/Game/UI/WBP_HealthBar.HealthBar` (`self.HealthBarWidget`)) (`self.GetPercentHealth`)))

(event `self.OnDeath`
  (bind _returnvalue (`GameplayStatics.GetPlayerController` 0))
  (`|ExecutionSequence`
    (:`then_0`
      ;[1 1 1] Ajouter le widget de GameOver à l'écran
      (cast `PlayerController` (`self.GetController`))
      (bind _returnvalue_2 (`|CreateWidget` "/Game/UI/WBP_GameOver.WBP_GameOver_C"))
      (`UserWidget.AddToViewport` _returnvalue_2 0))
    (:`then_1`
      ;[1 1 1] Enlever le widget health bar de l'écran
      (`Widget.RemoveFromParent` (`self.HealthBarWidget`)))
    (:`then_2`
      ;[1 1 1] Afficher la souris pour permettre le click
      (`/Engine/EditorBlueprintResources/StandardMacros.IsValid` _returnvalue
        (:`Is Valid`
          (set `PlayerController.bShowMouseCursor` true _returnvalue))))))

(event `self.UpdateItemCount`
  (params (NewPotionCount :type String))
  (`TextBlock.SetText` (`/Game/UI/WBP_Potions.TxtPotionCount` (`self.PotionWidget`)) (`KismetTextLibrary.Conv_StringToText` NewPotionCount)))

(fn `UserConstructionScript`)